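; Player inventory component that handles slot drops and keeps the owning player's item slots in sync with inventory changes.
; Drops from a Player Inventory or Player Hotbar container call TransferItem on the source, targeting this component at the dropped index.
; Add and remove overrides run the parent logic, then message the controller obtained from the owner to update or reset the affected slot.
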(fn HandleSlotDrop
  (params (Container :type BPC%20Items%20Container%20Object%20Reference) (FromIndex :type Integer) (DroppedIndex :type Integer))
  (LocalVariables|SetLocalFromContainer Container)
  (LocalVariables|SetLocalFromIndex FromIndex)
  (LocalVariables|SetLocalDroppedIndex DroppedIndex)
  (switch Utilities|FlowControl|Switch|SwitchonE_ContainerType (Variables|/Game/_Main/Blueprints/Inventory/BPC_ItemsContainer.BPC_ItemsContainer_C|GetContainerType (LocalVariables|GetLocalFromContainer))
    (:NewEnumerator0
      _)
    (:NewEnumerator1
      _))
  (Default|TransferItem (LocalVariables|GetLocalFromContainer) self (LocalVariables|GetLocalDroppedIndex) (LocalVariables|GetLocalFromIndex))
  (return))

(fn AddItemtoIndex
  (params (Item :type ST%20Item%20Info%20Structure) (LocalSpecificIndex :type Integer) (FromIndex :type Integer))
  (bind _success_ (|CallParentFunction Item LocalSpecificIndex FromIndex))
  (bind _controllerref (Class|BPISurvivalCharacter|GetControllerfromCharacter(Message) (Components|GetOwner)))
  (Default|UpdateItemSlot _controllerref (Variables|Default|GetContainerType) LocalSpecificIndex (CallFunction|GetItematIndex LocalSpecificIndex))
  (return _success_))

(fn RemoveItematIndex
  (params (Index :type Integer))
  (bind _success_ (|CallParentFunction Index))
  (bind _controllerref (Class|BPISurvivalCharacter|GetControllerfromCharacter(Message) (Components|GetOwner)))
  (Default|ResetItemSlot _controllerref (Variables|Default|GetContainerType) Index)
  (return _success_))