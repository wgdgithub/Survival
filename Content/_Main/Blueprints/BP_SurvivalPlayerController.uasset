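; Player controller for a survival game that owns the main HUD widget and handles the inventory UI.
; BeginPlay adds the default Enhanced Input mapping and creates the main widget only where the controller lacks authority (remote clients).
; Tab or I toggles the inventory, cursor and input mode.
; Slot update and reset events resolve widgets by container type and index; only inventory and hotbar are wired, not storage or armor.
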(event Custom|InventoryOnClient
  (if (Variables|Default|GetInventoryShow?)
    (Default|SetInventoryVisibility (Variables|Default|GetMainWidgetRef) false)
    (Variables|Default|SetbShowMouseCursor false)
    (Input|SetInputModeGameOnly self false)
    (Variables|Default|SetInventoryShow? false)
    (else
      (Default|SetInventoryVisibility (Variables|Default|GetMainWidgetRef) true)
      (Variables|Default|SetbShowMouseCursor true)
      (Input|SetInputModeGameandUI self 0 "DoNotLock" true false)
      (Variables|Default|SetInventoryShow? true))))

(event Custom|ResetItemSlot
  (params (Container :type E_ContainerType%20Enum :default "NewEnumerator0") (Index :type Integer))
  (bind _widget (CallFunction|GetInventoryWidget Container Index))
  (Utilities|IsValid _widget
    (:Is%20Valid
      (Default|ResetSlot _widget))))

(event Custom|UpdateItemSlot
  (params (Container :type E_ContainerType%20Enum :default "NewEnumerator0") (Index :type Integer) (ItemInfo :type ST%20Item%20Info%20Structure))
  (bind _widget (CallFunction|GetInventoryWidget Container Index))
  (Utilities|IsValid _widget
    (:Is%20Valid
      (Default|UpdateSlot _widget ItemInfo))))

(event EventBeginPlay
  (bind _returnvalue (PlayerController|LocalPlayerSubsystems|GetEnhancedInputLocalPlayerSubsystem))
  (Utilities|IsValid _returnvalue
    (:Is%20Valid
      (Input|AddMappingContext _returnvalue "/Game/FirstPerson/Input/IMC_Default.IMC_Default" 0 "(bIgnoreAllPressedKeysUntilRelease=True,bForceImmediately=False,bNotifyUserSettings=False)")
      ;[1 1 1] 只在客户端创建控件
      (Networking|SwitchHasAuthority
        (:Remote
          (bind _returnvalue_2 (UserInterface|CreateWidget "/Game/_Main/Widgets/WBP_MainWidget.WBP_MainWidget_C" self))
          (bind _output_get (Variables|Default|SetMainWidgetRef _returnvalue_2))
          (UserInterface|Viewport|AddtoViewport _output_get 0))))))

(event Input|KeyboardEvents|Tab
  (params (Key :type Key%20Structure :default "None"))
  (:Pressed
    (CallFunction|InventoryonClient)))

(event Input|KeyboardEvents|I
  (params (Key :type Key%20Structure :default "None"))
  (:Pressed
    (CallFunction|InventoryonClient)))

(fn ConstructionScript)

(fn GetInventoryWidget
  (params (Container :type E_ContainerType%20Enum :default "NewEnumerator0") (SlotIndex :type Integer))
  (bind _mainwidgetref (Variables|Default|GetMainWidgetRef))
  (return (Utilities|Array|Get(acopy) (Variables|/Game/_Main/Widgets/InventoryWidgets/WBP_ItemContainerGrid.WBP_ItemContainerGrid_C|GetSlots (Utilities|Select :Index Container :NewEnumerator0 (Variables|/Game/_Main/Widgets/InventoryWidgets/WBP_Inventory.WBP_Inventory_C|GetWBP_ItemContainerGrid (Variables|/Game/_Main/Widgets/WBP_MainWidget.WBP_MainWidget_C|GetWBP_Inventory _mainwidgetref)) :NewEnumerator1 (Variables|/Game/_Main/Widgets/InventoryWidgets/WBP_HotBar.WBP_HotBar_C|GetWBP_ItemContainerGrid (Variables|/Game/_Main/Widgets/WBP_MainWidget.WBP_MainWidget_C|GetWBP_HotBar _mainwidgetref)) :NewEnumerator2 0 :NewEnumerator3 0)) SlotIndex)))

(fn SurvivalPlayerControllerRef
  (return self))